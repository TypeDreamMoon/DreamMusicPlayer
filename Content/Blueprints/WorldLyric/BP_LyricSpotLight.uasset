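; BP_LyricSpotLight is a spot light Blueprint in WorldLyric with an UpdateColor event that is currently empty.
; An unconnected LinearColorTo chain would tween the light from its current color over one second through UpdateColorHandle, which sets the SpotLightComponent color.
; That chain brightens the target color by adding gray when any RGB channel is below one half, but it never runs.
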(event Custom|UpdateColor
  (params (Color :type Linear%20Color%20Structure)))

(event Custom|UpdateColorHandle
  (params (value :type Linear%20Color%20Structure%20%28by%20ref%29))
  (Rendering|Components|Light|SetLightColor (Variables|Default|GetSpotLightComponent) value true))

(fn ConstructionScript)