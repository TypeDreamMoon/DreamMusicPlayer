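; World lyric manager that drives in-world lyric actors, lights and a background mesh from a Dream Music Player.
; Initialize binds to player and expansion events; lyric changes rotate round-robin through LyricActors, and music ticks feed line progress to the active actor.
; Theme color changes give each light a random palette color.
; Track changes put the cover on the background's dynamic material and pass the Misc data's display type to lyric widgets.
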(event Custom|MusicTick
  (params (Time :type Float%20%28single-precision%29))
  (bind _mp (Variables|Default|GetMP))
  (bind _active (Variables|Default|GetActive)
    (:then
      (Default|TickLyric _active (.lineprogress (Class|DreamMusicPlayerExpansionLyric|GetCurrentLyricWordProgress (Class|DreamMusicPlayerComponent|GetExpansionbyClass _mp "/Script/DreamMusicPlayer.DreamMusicPlayerExpansion_Lyric") (Variables|/Script/DreamMusicPlayer.DreamMusicPlayerComponent|GetCurrentTimestamp _mp)))))
    (:else)))

(event Custom|Initialize
  (params (MusicPlayer :type Dream%20Music%20Player%20Component%20Object%20Reference))
  (bind _output_get (Variables|Default|SetMP MusicPlayer))
  (EventDispatchers|AssignOnLyricChanged (Class|DreamMusicPlayerComponent|GetExpansionbyClass _output_get "/Script/DreamMusicPlayer.DreamMusicPlayerExpansion_Lyric") (EventDispatchers|CreateEvent :!event Custom|LyricChanged))
  (EventDispatchers|BindEventtoOnMusicTick _output_get (EventDispatchers|CreateEvent :!event Custom|MusicTick))
  (Variables|Default|SetCurrentIndex 0)
  (EventDispatchers|BindEventtoOnThemeColorChanged (Class|DreamMusicPlayerComponent|GetExpansionbyClass _output_get "/Script/DreamMusicPlayer.DreamMusicPlayerExpansion_ThemeColors") (EventDispatchers|CreateEvent :!event Custom|OnThemeColorChanged))
  (EventDispatchers|BindEventtoOnMusicDataChanged _output_get (EventDispatchers|CreateEvent :!event Custom|MusicChanged))
  (bind _returnvalue (Rendering|Material|CreateDynamicMaterialInstance (Variables|/Script/Engine.StaticMeshActor|GetStaticMeshComponent (Variables|Default|GetBackground)) 0 "/Game/Materials/M_WD_BG.M_WD_BG" "None" :!class /Script/Engine.PrimitiveComponent))
  (Variables|Default|SetDMI _returnvalue))

(event Custom|LyricChanged
  (params (Lyric :type Dream%20Music%20Lyric%20Structure) (Index :type Integer))
  (Default|Changed (Utilities|Array|Get(acopy) (Variables|Default|GetLyricActors) (Variables|Default|GetCurrentIndex)) Lyric)
  (Variables|Default|SetActive (Utilities|Array|Get(acopy) (Variables|Default|GetLyricActors) (Variables|Default|GetCurrentIndex)))
  (bind _result (Math|Integer|IncrementInt (Variables|Default|GetCurrentIndex))
    (:%20%20
      (if (not (Utilities|Array|IsValidIndex (Variables|Default|GetLyricActors) _result))
        (Variables|Default|SetCurrentIndex 0)))))

(event Custom|Deinitialized
  (bind _mp (Variables|Default|GetMP))
  (Utilities|IsValid _mp
    (:Is%20Valid
      (EventDispatchers|UnbindEventfromOnLyricChanged (Class|DreamMusicPlayerComponent|GetExpansionbyClass _mp "/Script/DreamMusicPlayer.DreamMusicPlayerExpansion_Lyric") (EventDispatchers|CreateEvent :!event Custom|LyricChanged)))))

(event Custom|OnThemeColorChanged
  (params (Colors :type Array%20of%20K%20Means%20Color%20Cluster%20Structures) (bSuccess :type Boolean))
  (for _array_element (Variables|Default|GetLights)
    (Default|UpdateColor _array_element (.color (.OutItem (Utilities|Array|Random Colors))))))

(event Custom|MusicChanged
  (params (Data :type Dream%20Music%20Data%20Struct%20Structure))
  (Rendering|Material|SetTextureParameterValue (Variables|Default|GetDMI) "Texture" (Variables|/Script/DreamMusicPlayer.DreamMusicPlayerComponent|GetCover (Variables|Default|GetMP)))
  (bind _array_element (Utilities|Array|ForEachLoopwithBreak (.expansiondatas Data) :!label _label)
    (:LoopBody
      (if (== (Utilities|GetClass _array_element) "/Game/Blueprints/DMPED_Misc.DMPED_Misc_C")
        (for _array_element_2 (Variables|Default|GetLyricActors)
          (Default|Initilaize (Variables|/Game/Blueprints/WorldLyric/BP_LyricActor.BP_LyricActor_C|GetWorldUI _array_element_2) (Variables|/Game/Blueprints/DMPED_Misc.DMPED_Misc_C|GetDisplayType (.AsDMPED%20Misc (Utilities|Casting|CastToDMPED_Misc _array_element)))))
        (goto _label Break)))))

(fn ConstructionScript)