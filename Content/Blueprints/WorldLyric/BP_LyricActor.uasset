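; BP_LyricActor is a world-placed lyric display for the music player, showing lyrics through a W_WorldMusicPlayer_Lyric widget cached on BeginPlay.
; When the lyric changes, it blends the player view to its Camera with a short cubic blend, sends the line to the widget and plays a Level Sequence through a newly created player.
; TickLyric forwards playback progress to the widget.
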(event Custom|Changed
  (params (Lyric :type Dream%20Music%20Lyric%20Structure))
  (Game|Player|SetViewTargetwithBlend (Game|GetPlayerController 0) (Variables|Default|GetCamera) 0.25 "VTBlend_Cubic" 0.0 false)
  (Default|SetLyric (Variables|Default|GetWorldUI) Lyric)
  (bind _returnvalue (Sequencer|Player|CreateLevelSequencePlayer (Variables|Default|GetLS) (Variables|Default|GetSettings)))
  (Sequencer|Player|Play _returnvalue :!class /Script/MovieScene.MovieSceneSequencePlayer))

(event Custom|TickLyric
  (params (Progress :type Float%20%28double-precision%29))
  (Default|TickLyric (Variables|Default|GetWorldUI) Progress))

(event EventBeginPlay
  (bind _asw_world_music_player_lyric (Utilities|Casting|CastToW_WorldMusicPlayer_Lyric (UserInterface|GetWidget (Variables|Default|GetWidget))))
  (Variables|Default|SetWorldUI _asw_world_music_player_lyric))

(fn ConstructionScript)