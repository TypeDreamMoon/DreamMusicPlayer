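; Lyric event definition for DreamMusicPlayer that drives film grain on a PostProcessVolume found in the level.
; TWEEN_NOISE stores a bool payload as a flag that NOISE checks.
; With the flag on, NOISE tweens grain intensity from its current value to the float payload over a fixed duration.
; With it off, NOISE sets the grain to zero immediately, ignoring the payload value.
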(event Custom|TWEEN_NOISE
  (params (Lyric :type Dream%20Music%20Lyric%20Structure) (EventPayload :type Dream%20Music%20Player%20Payload%20Object%20Reference))
  (bind _asbool_payload (Utilities|Casting|CastToDreamMusicPlayerPayload_Bool EventPayload))
  (Variables|Default|SetbTweenNoise (Variables|/Script/DreamMusicPlayer.DreamMusicPlayerPayload_Bool|GetValue _asbool_payload)))

(event Custom|NOISE
  (params (Lyric :type Dream%20Music%20Lyric%20Structure) (EventPayload :type Dream%20Music%20Player%20Payload%20Object%20Reference))
  (bind _asfloat_payload (Utilities|Casting|CastToDreamMusicPlayerPayload_Float EventPayload))
  (bind _returnvalue (Actor|GetActorOfClass "/Script/Engine.PostProcessVolume"))
  (if (Variables|Default|GetbTweenNoise)
    (Class|LTweenBPLibrary|Floatto (delegate Custom|OnTweenNoise) (Utilities|Struct|BreakPostProcessSettings (Variables|/Script/Engine.PostProcessVolume|GetSettings _returnvalue)) (Variables|/Script/DreamMusicPlayer.DreamMusicPlayerPayload_Float|GetValue _asfloat_payload) 2.0)
    (else
      (bind _structout (Utilities|Struct|SetmembersinPostProcessSettings (Variables|/Script/Engine.PostProcessVolume|GetSettings _returnvalue) 0.0))
      (Variables|/Script/Engine.PostProcessVolume|SetSettings _returnvalue _structout))))

(event Custom|OnTweenNoise
  (params (value :type Float%20%28single-precision%29))
  (bind _structout (Utilities|Struct|SetmembersinPostProcessSettings (Variables|/Script/Engine.PostProcessVolume|GetSettings (stale Custom|NOISE _returnvalue)) value))
  (Variables|/Script/Engine.PostProcessVolume|SetSettings (stale Custom|NOISE _returnvalue) _structout))